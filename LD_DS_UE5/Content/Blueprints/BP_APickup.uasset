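; Base pickup actor that reacts to an interact event and holds a HUD reference for updating on pickup.
; On BeginPlay it caches the ThirdPersonGameMode and, after a short delay, takes the HUD reference from it.
; Interacting calls CheckHUDBox, an empty function here, plays an ammo pickup sound, then destroys the static and skeletal mesh components if both are valid, leaving the actor itself alive.
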(event EventBeginPlay
  (|CallParentFunction)
  (bind _asthird_person_game_mode (Utilities|Casting|CastToThirdPersonGameMode (Game|GetGameMode)))
  (bind _output_get (Variables|Default|SetGameModeRef _asthird_person_game_mode))
  (Utilities|FlowControl|Delay 0.2)
  (Variables|Default|SetHUD%20Ref (Variables|/Game/Blueprints/ThirdPersonGameMode.ThirdPersonGameMode_C|GetHUDRef _output_get)))

(event Collision|EventActorBeginOverlap
  (params (OtherActor :type Actor%20Object%20Reference))
  (|CallParentFunction OtherActor) ; This node is disabled and will not be called.\nDrag off pins to build functionality.
)

(event EventTick
  (params (DeltaSeconds :type Float%20%28single-precision%29))
  (|CallParentFunction DeltaSeconds) ; This node is disabled and will not be called.\nDrag off pins to build functionality.
)

(event EventOnStartInteract
  (bind _staticmesh (Variables|Default|GetStaticMesh))
  (CallFunction|CheckHUDBox)
  (Audio|PlaySound2D "/Game/Resources/Audio/Gun_Ammo_Pickup06_Cue.Gun_Ammo_Pickup06_Cue" 1.0 1.0 0.0 0 0)
  (Utilities|IsValid _staticmesh
    (:Is%20Valid
      (Utilities|IsValid (Variables|Default|GetSkeletalMesh)
        (:Is%20Valid
          (Components|DestroyComponent _staticmesh))))))

(fn ConstructionScript
  (|CallParentFunction))

(fn CheckHUDBox)