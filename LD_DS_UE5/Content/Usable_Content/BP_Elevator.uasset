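; Usable elevator actor that moves its center mesh between a bottom and a top point, toggling direction on each interaction.
; SetupElevator runs at construction and BeginPlay, placing the top point by a height offset and fitting the trigger box to the shaft.
; It also scales the timeline play rate inversely with travel distance for consistent speed.
; Interacting plays a click sound and flip-flops the timeline forward or backward, lerping the mesh's position.
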(event EventBeginPlay
  (|CallParentFunction)
  (CallFunction|SetupElevator))

(event Collision|EventActorBeginOverlap
  (params (OtherActor :type Actor%20Object%20Reference))
  (|CallParentFunction OtherActor) ; This node is disabled and will not be called.\nDrag off pins to build functionality.
)

(event EventTick
  (params (DeltaSeconds :type Float%20%28single-precision%29))
  (|CallParentFunction DeltaSeconds) ; This node is disabled and will not be called.\nDrag off pins to build functionality.
)

(event EventOnStartInteract
  (Audio|PlaySound2D "/Engine/VREditor/Sounds/UI/Click_on_Button_Cue.Click_on_Button_Cue" 1.0 1.0 0.0 0 0)
  (Utilities|FlowControl|FlipFlop
    (:A
      (bind _alpha (Timeline|ElevatorTimeline Play)
        (:Update
          (Transformation|SetWorldLocation (Variables|Default|GetCenterElevatorMesh) (Math|Vector|Lerp(Vector) (Transformation|GetWorldLocation (Variables|Default|GetButtom)) (Transformation|GetWorldLocation (Variables|Default|GetTop)) _alpha) false false))))
    (:B
      (Timeline|ElevatorTimeline Reverse))))

(fn ConstructionScript
  (|CallParentFunction)
  (CallFunction|SetupElevator))

(fn SetupElevator
  (bind _buttom (Variables|Default|GetButtom))
  (bind _uppos (Variables|Default|GetUpPos))
  (bind _triggerbox (Variables|Default|GetTriggerBox))
  (bind _returnvalue (Transformation|GetWorldLocation _buttom))
  (bind _boxextent (Variables|/Script/Engine.BoxComponent|GetBoxExtent _triggerbox))
  (bind _returnvalue_2 (+ (Math|Vector|MakeVector 0.0 0.0 _uppos) _returnvalue))
  (bind _returnvalue_3 (Math|Vector|Distance(Vector) _returnvalue_2 _returnvalue))
  (Transformation|SetWorldLocation (Variables|Default|GetTriggerBox) (+ (/ (- _returnvalue_2 _returnvalue) 2) _returnvalue) false false)
  (Transformation|SetWorldLocation (Variables|Default|GetTop) _returnvalue_2 false false)
  (Components|Box|SetBoxExtent _triggerbox (Math|Vector|MakeVector (.x _boxextent) (.y _boxextent) (+ (/ _returnvalue_3 2.0) 1e+02)) true)
  (Components|Timeline|SetPlayRate (Variables|Default|GetElevatorTimeline) (* (/ 1.0 (/ _returnvalue_3 1e+02)) (Variables|Default|GetElevatorSpeed))))