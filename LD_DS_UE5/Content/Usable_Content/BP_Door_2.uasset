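; BP_Door_2 is an interactable door that can be locked or opened.
; On interact start it checks a LockedDoor flag: a locked door plays a handle-rattle sound.
; An unlocked door destroys its DoorMesh component instead of animating it, then plays an opening sound.
; Both sounds play as non-spatialized 2D audio.
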(event EventBeginPlay
  (|CallParentFunction) ; This node is disabled and will not be called.\nDrag off pins to build functionality.
)

(event Collision|EventActorBeginOverlap
  (params (OtherActor :type Actor%20Object%20Reference))
  (|CallParentFunction OtherActor) ; This node is disabled and will not be called.\nDrag off pins to build functionality.
)

(event EventTick
  (params (DeltaSeconds :type Float%20%28single-precision%29))
  (|CallParentFunction DeltaSeconds) ; This node is disabled and will not be called.\nDrag off pins to build functionality.
)

(event EventOnStartInteract
  (if (Variables|Default|GetbLockedDoor)
    (Audio|PlaySound2D "/Game/Resources/Audio/Door_Locked_HandleRattle3_Cue.Door_Locked_HandleRattle3_Cue" 1.0 1.0 0.0 0 0)
    (else
      (Components|DestroyComponent (Variables|Default|GetDoorMesh))
      (Audio|PlaySound2D "/Game/Resources/Audio/SFX_OpenDoor_01_Cue.SFX_OpenDoor_01_Cue" 1.0 1.0 0.0 0 0))))

(fn ConstructionScript
  (|CallParentFunction))