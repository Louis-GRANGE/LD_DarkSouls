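; BP_LockedDoor is an actor that pairs a door with a button that unlocks it.
; On BeginPlay it casts its Door and Button child actors to BP_Door and BP_AButton, marks the door locked and binds to the button's start-interact event.
; The first button interaction plays a 2D door-opening sound and clears the door's locked flag, with a DoOnce preventing repeats.
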(event Custom|InteractWithButton
  (Utilities|FlowControl|DoOnce false
    (:Completed
      (Audio|PlaySound2D "/Game/Resources/Audio/SFX_OpenDoor_04_Cue.SFX_OpenDoor_04_Cue" 1.0 1.0 0.0 0 0)
      (Variables|/Game/Usable_Content/BP_Door.BP_Door_C|SetbLockedDoor (Variables|Default|GetDoorRef) false))))

(event EventBeginPlay
  (bind _asbp_door (Utilities|Casting|CastToBP_Door (Variables|/Script/Engine.ChildActorComponent|GetChildActor (Variables|Default|GetDoor))))
  (bind _output_get (Variables|Default|SetDoorRef _asbp_door))
  (Variables|/Game/Usable_Content/BP_Door.BP_Door_C|SetbLockedDoor _output_get true)
  (bind _asbp_abutton (Utilities|Casting|CastToBP_AButton (Variables|/Script/Engine.ChildActorComponent|GetChildActor (Variables|Default|GetButton))))
  (bind _output_get_2 (Variables|Default|SetButtonRef _asbp_abutton))
  (EventDispatchers|BindEventtoDelegateonStartInteract _output_get_2 (delegate Custom|InteractWithButton)))

(event Collision|EventActorBeginOverlap
  (params (OtherActor :type Actor%20Object%20Reference)))

(event EventTick
  (params (DeltaSeconds :type Float%20%28single-precision%29)))

(fn ConstructionScript)